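; BP_Copter is a roaming helicopter that randomly drops power-ups at its position.
; From BeginPlay it loops AI moves to random navigable points, adjusting yaw after each successful move and retrying on failure.
; Tick uses a Delay as a repeating timer for cascading random rolls that spawn QuackHole or EMP pickups, print a Cattle Prod placeholder, or do nothing.
; Tick also spins the blade pivot by RPM scaled with delta time.
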(event `FlyRandomly_Event`
  (bind (_returnvalue_roll _returnvalue_pitch _returnvalue_yaw) (`KismetMathLibrary.BreakRotator` (`self.K2_GetActorRotation`)))
  (bind _randomlocation (`NavigationSystemV1.K2_GetRandomLocationInNavigableRadius` (`self.K2_GetActorLocation`) 5000.0 null null :!label _label))
  (`|AIMoveTo` self _randomlocation null
    (:`OnSuccess`
      (bind (_returnvalue_roll_2 _returnvalue_pitch_2 _returnvalue_yaw_2) (`KismetMathLibrary.BreakRotator` (`KismetMathLibrary.FindLookAtRotation` (`self.K2_GetActorLocation`) _randomlocation)))
      (`self.K2_SetActorRotation` (`KismetMathLibrary.MakeRotator` 0.0 0.0 (- _returnvalue_yaw_2 _returnvalue_yaw)))
      (`KismetSystemLibrary.Delay` 1.0)
      (`self.FlyRandomly_Event`))
    (:`OnFail`
      (`self.FlyRandomly_Event`))))

(event `self.ReceiveBeginPlay`
  (goto _label))

(event `self.ReceiveTick`
  (params (DeltaSeconds :type "Float (single-precision)"))
  (bind _returnvalue (* (`KismetMathLibrary.RandomFloat`) 100.0))
  (`|ExecutionSequence`
    (:`then_0`
      (`KismetSystemLibrary.Delay` 5.0)
      (if (> _returnvalue 90.0)
        (`|SpawnActorFromClass` "/Game/Blueprints/BP_PowerUp_QuackHole.BP_PowerUp_QuackHole_C" (`self.GetTransform`) "Undefined" "MultiplyWithRoot" null null)
        (elif (> _returnvalue 70.0)
          (`KismetSystemLibrary.PrintString` "Cattle Prod")
          (elif (> _returnvalue 40.0)
            (`|SpawnActorFromClass` "/Game/Blueprints/BP_PowerUp_EMP.BP_PowerUp_EMP_C" (`self.GetTransform`) "Undefined" "MultiplyWithRoot" null null)))))
    (:`then_1`
      (`SceneComponent.K2_AddLocalRotation` (`self.BladePivotPoint`) (`KismetMathLibrary.MakeRotator` 0.0 0.0 (* DeltaSeconds (`self.RPM`))) false false))))

(fn `UserConstructionScript`)
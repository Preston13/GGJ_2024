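; BP_Steak is a short-lived pickup that permanently multiplies the player character's walk speed by a small factor on overlap, then destroys itself.
; It expires after a random lifespan if not collected.
; Its GoToPlayer event starts a per-tick loop that pulls the physics box toward the player with acceleration-based force.
; On EndPlay, whether collected or expired, it decrements the player character's TotalSteakCount.
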(event `self.ReceiveBeginPlay`
  (`self.SetLifeSpan` (`KismetMathLibrary.RandomFloatInRange` 10.0 15.0)))

(event `self.Box.OnComponentBeginOverlap`
  (params (OverlappedComponent :type "PrimitiveComponent Object Reference") (OtherActor :type "Actor Object Reference") (OtherComp :type "PrimitiveComponent Object Reference") (OtherBodyIndex :type Integer) (bFromSweep :type Boolean) (SweepResult :type "HitResult Structure (by ref)"))
  (bind _asbp_third_person_character (cast `/Game/ThirdPerson/Blueprints/BP_ThirdPersonCharacter` OtherActor))
  (bind _charactermovement (`Character.CharacterMovement` _asbp_third_person_character))
  (set `CharacterMovementComponent.MaxWalkSpeed` (* (`CharacterMovementComponent.MaxWalkSpeed` _charactermovement) 1.05) _charactermovement)
  (`self.K2_DestroyActor`))

(event `GoToPlayer`
  (`PrimitiveComponent.AddForce` (`self.Box`) (* (`KismetMathLibrary.Normal` (- (`self.K2_GetActorLocation` (`GameplayStatics.GetPlayerPawn` 0)) (`self.K2_GetActorLocation`))) 1000.0) "None" true :!label _label)
  (`KismetSystemLibrary.DelayUntilNextTick`)
  (goto _label))

(event `self.ReceiveEndPlay`
  (params (EndPlayReason :type "EEndPlayReason Enum" :default "Destroyed"))
  (bind _asbp_third_person_character (cast `/Game/ThirdPerson/Blueprints/BP_ThirdPersonCharacter` (`GameplayStatics.GetPlayerPawn` 0)))
  (`/Engine/EditorBlueprintResources/StandardMacros.DecrementInt` (`/Game/ThirdPerson/Blueprints/BP_ThirdPersonCharacter.TotalSteakCount` _asbp_third_person_character)))

(fn `UserConstructionScript`)
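; Spawner actor that populates the level with enemy alien ships and a copter on a scripted timeline after BeginPlay.
; A single chain of Delay nodes fires five one-shot spawns: four BP_AlienShip and one BP_Copter midway through, with no looping.
; Each spawn picks a random navigable point within a large radius of the spawner, adjusting for collisions but always spawning.
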(event `self.ReceiveBeginPlay`
  (`KismetSystemLibrary.Delay` 3.0)
  (bind _randomlocation (`NavigationSystemV1.K2_GetRandomLocationInNavigableRadius` (`self.K2_GetActorLocation`) 8000.0 null null))
  (`|SpawnActorFromClass` "/Game/Blueprints/BP_AlienShip.BP_AlienShip_C" (`KismetMathLibrary.Conv_VectorToTransform` _randomlocation) "AdjustIfPossibleButAlwaysSpawn" "MultiplyWithRoot" null null)
  (`KismetSystemLibrary.Delay` 10.0)
  (bind _randomlocation_2 (`NavigationSystemV1.K2_GetRandomLocationInNavigableRadius` (`self.K2_GetActorLocation`) 8000.0 null null))
  (`|SpawnActorFromClass` "/Game/Blueprints/BP_AlienShip.BP_AlienShip_C" (`KismetMathLibrary.Conv_VectorToTransform` _randomlocation_2) "AdjustIfPossibleButAlwaysSpawn" "MultiplyWithRoot" null null)
  (`KismetSystemLibrary.Delay` 2.0)
  (bind _randomlocation_3 (`NavigationSystemV1.K2_GetRandomLocationInNavigableRadius` (`self.K2_GetActorLocation`) 8000.0 null null))
  (`|SpawnActorFromClass` "/Game/Blueprints/BP_Copter.BP_Copter_C" (`KismetMathLibrary.Conv_VectorToTransform` _randomlocation_3) "AdjustIfPossibleButAlwaysSpawn" "MultiplyWithRoot" null null)
  (`KismetSystemLibrary.Delay` 5.0)
  (bind _randomlocation_4 (`NavigationSystemV1.K2_GetRandomLocationInNavigableRadius` (`self.K2_GetActorLocation`) 8000.0 null null))
  (`|SpawnActorFromClass` "/Game/Blueprints/BP_AlienShip.BP_AlienShip_C" (`KismetMathLibrary.Conv_VectorToTransform` _randomlocation_4) "AdjustIfPossibleButAlwaysSpawn" "MultiplyWithRoot" null null)
  (`KismetSystemLibrary.Delay` 5.0)
  (bind _randomlocation_5 (`NavigationSystemV1.K2_GetRandomLocationInNavigableRadius` (`self.K2_GetActorLocation`) 8000.0 null null))
  (`|SpawnActorFromClass` "/Game/Blueprints/BP_AlienShip.BP_AlienShip_C" (`KismetMathLibrary.Conv_VectorToTransform` _randomlocation_5) "AdjustIfPossibleButAlwaysSpawn" "MultiplyWithRoot" null null))

(fn `UserConstructionScript`)
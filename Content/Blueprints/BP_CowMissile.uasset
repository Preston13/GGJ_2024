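; BP_CowMissile is a homing projectile that chases the player and knocks them down on contact.
; After a short delay, a per-tick loop applies mass-independent force to its mesh toward the player pawn.
; On first overlap with the third-person character, it plays a dead-cow sound, ragdolls them and shows a steak-collection hint.
; It then destroys the player's crate, or spawns BP_ExplodingActors if none is held, and destroys itself.
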(event `self.ReceiveBeginPlay`
  (`KismetSystemLibrary.Delay` 0.1)
  (`PrimitiveComponent.AddForce` (`self.StaticMesh`) (* (`KismetMathLibrary.Normal` (- (`self.K2_GetActorLocation` (`GameplayStatics.GetPlayerPawn` 0)) (`self.K2_GetActorLocation`))) 5000.0) "None" true :!label _label)
  (`KismetSystemLibrary.DelayUntilNextTick`)
  (goto _label))

(event `self.Collider.OnComponentBeginOverlap`
  (params (OverlappedComponent :type "PrimitiveComponent Object Reference") (OtherActor :type "Actor Object Reference") (OtherComp :type "PrimitiveComponent Object Reference") (OtherBodyIndex :type Integer) (bFromSweep :type Boolean) (SweepResult :type "HitResult Structure (by ref)"))
  (bind (_returnvalue_location _returnvalue_rotation) (`KismetMathLibrary.BreakTransform` (`self.GetTransform`)))
  (bind _asbp_third_person_character (cast `/Game/ThirdPerson/Blueprints/BP_ThirdPersonCharacter` OtherActor))
  (`/Engine/EditorBlueprintResources/StandardMacros.DoOnce` false
    (:`Completed`
      (bind _returnvalue (`self.K2_GetActorLocation` _asbp_third_person_character))
      (`GameplayStatics.PlaySoundAtLocation` "/Game/Sound_Effects_from_Free_Sound/Cow_Moos/431860__cheetahzbrain__dead-cow.431860__cheetahzbrain__dead-cow" _returnvalue (struct) 1.0 1.0 0.0 null null null null)
      (`/Game/ThirdPerson/Blueprints/BP_ThirdPersonCharacter.Ragdoll` _asbp_third_person_character)
      (`/Game/ThirdPerson/Blueprints/BP_ThirdPersonCharacter.DisplayHUDMessage` _asbp_third_person_character "Collect the steaks to increase speed!")
      (if (`/Game/ThirdPerson/Blueprints/BP_ThirdPersonCharacter.bHasCrate` _asbp_third_person_character)
        (`/Game/ThirdPerson/Blueprints/BP_ThirdPersonCharacter.DestroyCrate` _asbp_third_person_character)
        (else
          (`|SpawnActorFromClass` "/Game/Blueprints/BP_ExplodingActors.BP_ExplodingActors_C" (`KismetMathLibrary.MakeTransform` _returnvalue _returnvalue_rotation) "AlwaysSpawn" "MultiplyWithRoot" null null)))
      (`self.K2_DestroyActor`))))

(event `self.ReceiveHit`
  (params (MyComp :type "PrimitiveComponent Object Reference") (Other :type "Actor Object Reference") (OtherComp :type "PrimitiveComponent Object Reference") (bSelfMoved :type Boolean) (HitLocation :type "Vector Structure") (HitNormal :type "Vector Structure") (NormalImpulse :type "Vector Structure") (Hit :type "HitResult Structure (by ref)")))

(fn `UserConstructionScript`)
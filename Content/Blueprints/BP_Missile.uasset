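; BP_Missile is a projectile actor that flies at the spot where the player stood when it spawned, without homing.
; BeginPlay caches the player pawn's location and turns to face it.
; Tick lerps from its current location toward just below that point with a growing alpha, speeding up the approach.
; Past a small alpha threshold, it enables physics and gravity on the Missile component and clears IsDeadly.
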(event `self.ReceiveBeginPlay`
  (bind _output_get (set `self.PlayerLocation` (`self.K2_GetActorLocation` (`GameplayStatics.GetPlayerPawn` 0))))
  (`self.K2_SetActorRotation` (`KismetMathLibrary.FindLookAtRotation` (`self.K2_GetActorLocation`) _output_get)))

(event `self.ReceiveTick`
  (params (DeltaSeconds :type "Float (single-precision)"))
  (bind _missile (`self.Missile`))
  (set `self.Alpha` (+ (`self.Alpha`) (/ DeltaSeconds 10.0)))
  (`self.K2_SetActorLocation` (`KismetMathLibrary.VLerp` (`self.K2_GetActorLocation`) (- (`self.PlayerLocation`) (0.0 0.0 25.0)) (`self.Alpha`)))
  (if (>= (`self.Alpha`) 0.15)
    (`PrimitiveComponent.SetSimulatePhysics` _missile true)
    (`PrimitiveComponent.SetEnableGravity` _missile true)
    (set `self.IsDeadly` false)))

(fn `UserConstructionScript`)
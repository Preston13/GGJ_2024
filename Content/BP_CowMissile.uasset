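; BP_CowMissile is a homing cow projectile that knocks down the player on contact.
; A looping timer started at BeginPlay drives physics-based homing, applying acceleration-mode force to the mesh toward the player pawn.
; On first overlap with the third-person character, it plays a sound, ragdolls them and shows a steak-collection hint.
; It then destroys their crate, or spawns BP_ExplodingActors if they have none, and destroys itself.
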(event `self.ReceiveBeginPlay`
  (bind _returnvalue (`GameplayStatics.GetPlayerPawn` 0))
  (`/Engine/EditorBlueprintResources/StandardMacros.IsValid` _returnvalue
    (:`Is Valid`
      (set `self.Player` _returnvalue)
      (bind _returnvalue_2 (`KismetSystemLibrary.K2_SetTimerDelegate` (`|CreateDelegate` :!event `ProjectileMovement`) (`GameplayStatics.GetWorldDeltaSeconds`) true 0.1))
      (set `self.ProjectileMovementTimer` _returnvalue_2))))

(event `ProjectileMovement`
  (`/Engine/EditorBlueprintResources/StandardMacros.IsValid` (`self.Player`)
    (:`Is Valid`
      (`PrimitiveComponent.AddForce` (`self.StaticMesh`) (* (`KismetMathLibrary.Normal` (- (`self.K2_GetActorLocation` (`GameplayStatics.GetPlayerPawn` 0)) (`self.K2_GetActorLocation`))) (`self.ProjectileMovementForce`)) "None" true))))

(event `self.Collider.OnComponentBeginOverlap`
  (params (OverlappedComponent :type "PrimitiveComponent Object Reference") (OtherActor :type "Actor Object Reference") (OtherComp :type "PrimitiveComponent Object Reference") (OtherBodyIndex :type Integer) (bFromSweep :type Boolean) (SweepResult :type "HitResult Structure (by ref)"))
  (bind (_returnvalue_location _returnvalue_rotation) (`KismetMathLibrary.BreakTransform` (`self.GetTransform`)))
  (bind _asbp_third_person_character (cast `/Game/ThirdPerson/Blueprints/BP_ThirdPersonCharacter` OtherActor))
  (`/Engine/EditorBlueprintResources/StandardMacros.DoOnce` false
    (:`Completed`
      (`GameplayStatics.PlaySound2D` "/Game/Sound_Effects_from_Free_Sound/Cow_Moos/431860__cheetahzbrain__dead-cow.431860__cheetahzbrain__dead-cow" 1.0 1.0 0.0 null null)
      (`/Game/ThirdPerson/Blueprints/BP_ThirdPersonCharacter.Ragdoll` _asbp_third_person_character)
      (`/Game/ThirdPerson/Blueprints/BP_ThirdPersonCharacter.DisplayHUDMessage` _asbp_third_person_character "Collect the steaks to increase speed!")
      (if (`/Game/ThirdPerson/Blueprints/BP_ThirdPersonCharacter.bHasCrate` _asbp_third_person_character)
        (`/Game/ThirdPerson/Blueprints/BP_ThirdPersonCharacter.DestroyCrate` _asbp_third_person_character)
        (else
          (`|SpawnActorFromClass` "/Game/BP_ExplodingActors.BP_ExplodingActors_C" (`KismetMathLibrary.MakeTransform` (`self.K2_GetActorLocation` _asbp_third_person_character) _returnvalue_rotation) "AlwaysSpawn" "MultiplyWithRoot" null null)))
      (`self.K2_DestroyActor`))))

(fn `UserConstructionScript`)
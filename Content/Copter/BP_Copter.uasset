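; BP_Copter is an AI-moved pawn that wanders the navmesh, occasionally spawning cow missiles and quack holes.
; BeginPlay and FlyRandomly_Event share a move to a random reachable point nearby, re-invoking CallFlyRandomly right after issuing the move.
; A successful move has a coin-flip chance to spawn BP_CowMissile high above the copter and call it again.
; Tick uses a Delay to periodically roll a small chance of spawning BP_QuackHole in place.
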(event `FlyRandomly_Event`
  (bind _randomlocation (`NavigationSystemV1.K2_GetRandomLocationInNavigableRadius` (`self.K2_GetActorLocation`) 5000.0 null null :!label _label))
  (`|AIMoveTo` self _randomlocation null
    (:`then`
      (`self.FlyRandomly`))
    (:`OnSuccess`
      (if (> (`KismetMathLibrary.RandomFloat`) 0.5)
        (`|SpawnActorFromClass` "/Game/BP_CowMissile.BP_CowMissile_C" (`KismetMathLibrary.MakeTransform` (- (.location (`self.GetTransform`)) (0.0 0.0 -1500.0)) (.rotation (`self.GetTransform`))) "AlwaysSpawn" "MultiplyWithRoot" null null)
        (`self.FlyRandomly`)))))

(event `self.ReceiveBeginPlay`
  (goto _label))

(event `self.ReceiveTick`
  (params (DeltaSeconds :type "Float (single-precision)"))
  (`KismetSystemLibrary.Delay` 5.0)
  (if (> (* (`KismetMathLibrary.RandomFloat`) 100.0) 90.0)
    (`|SpawnActorFromClass` "/Game/BP_QuackHole.BP_QuackHole_C" (`self.GetTransform`) "Undefined" "MultiplyWithRoot" null null)))

(fn `UserConstructionScript`)
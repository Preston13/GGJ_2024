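; BP_AlienShip is an alien ship that roams the navmesh and randomly fires cow missiles.
; After a random startup delay, it loops FlyRandomly, using AI Move To toward a random navigable point around its current location.
; On arrival it may spawn a BP_CowMissile high above itself with a cannon sound, then pauses before moving again.
; A failed move retries immediately with a new destination.
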(event `FlyRandomly`
  (bind _location (.location (`self.GetTransform`)))
  (bind _randomlocation (`NavigationSystemV1.K2_GetRandomLocationInNavigableRadius` (`self.K2_GetActorLocation`) 5000.0 null null :!label _label))
  (`|AIMoveTo` self _randomlocation null
    (:`OnSuccess`
      (if (> (`KismetMathLibrary.RandomFloat`) 0.5)
        (`|SpawnActorFromClass` "/Game/BP_CowMissile.BP_CowMissile_C" (`KismetMathLibrary.MakeTransform` (- _location (0.0 0.0 -1500.0)) (.rotation (`self.GetTransform`))) "AlwaysSpawn" "MultiplyWithRoot" null null)
        (`GameplayStatics.PlaySoundAtLocation` "/Game/Sound_Effects_from_Free_Sound/Alien_Cannon/565449__newlocknew__plasma-cannon-shot_1-23lrsmltprcssng.565449__newlocknew__plasma-cannon-shot_1-23lrsmltprcssng" _location (struct) 1.0 1.0 0.0 null null null null))
      (`KismetSystemLibrary.Delay` 2.0)
      (`self.FlyRandomly`))
    (:`OnFail`
      (`self.FlyRandomly`))))

(event `self.ReceiveBeginPlay`
  (`KismetSystemLibrary.Delay` (`KismetMathLibrary.RandomFloatInRange` 2.0 5.0))
  (goto _label))

(fn `UserConstructionScript`)
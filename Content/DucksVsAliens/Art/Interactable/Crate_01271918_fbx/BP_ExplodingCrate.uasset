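; BP_ExplodingCrate is an interactable actor that spawns a cubic grid of BP_Duck actors at its location on BeginPlay.
; It spawns only if the player's BP_ThirdPersonCharacter is below its maximum duck count.
; SpawnActors runs three nested loops bounded by the rounded-up cube root of AmountToSpawn, offsetting each duck on an evenly spaced grid.
; Each spawn checks and increments the player's steak count, not the duck count.
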(event `self.ReceiveBeginPlay`
  (bind _asbp_third_person_character (cast `/Game/DucksVsAliens/Core/BP_ThirdPersonCharacter` (`GameplayStatics.GetPlayerPawn` 0)))
  (if (not (>= (`/Game/DucksVsAliens/Core/BP_ThirdPersonCharacter.TotalDuckCount` _asbp_third_person_character) (`/Game/DucksVsAliens/Core/BP_ThirdPersonCharacter.MaxDuckCount` _asbp_third_person_character)))
    (set `self.Player` _asbp_third_person_character)
    (`self.SpawnActors` (`self.AmountToSpawn`))))

(fn `SpawnActors`
  (params (AmountToSpawn :type Integer))
  (locals (X :type Integer) (Y :type Integer) (Z :type Integer))
  (bind _player (`self.Player`))
  (bind _totalsteakcount (`/Game/DucksVsAliens/Core/BP_ThirdPersonCharacter.TotalSteakCount` _player))
  (bind _returnvalue (`KismetMathLibrary.FCeil` (`KismetMathLibrary.MultiplyMultiply_FloatFloat` (`KismetMathLibrary.Conv_IntToDouble` AmountToSpawn) 0.333333)))
  (for _index (range (+ _returnvalue 1))
    (set `local.X` _index)
    (for _index_2 (range (+ _returnvalue 1))
      (set `local.Y` _index_2)
      (for _index_3 (range (+ _returnvalue 1))
        (set `local.Z` _index_3)
        (if (not (>= _totalsteakcount (`/Game/DucksVsAliens/Core/BP_ThirdPersonCharacter.MaxSteakCount` _player)))
          (`/Engine/EditorBlueprintResources/StandardMacros.IncrementInt` _totalsteakcount
            (:`  `
              (`|SpawnActorFromClass` "/Game/DucksVsAliens/Art/Interactable/Rubber_Duck/BP_Duck.BP_Duck_C" (`KismetMathLibrary.MakeTransform` (+ (`KismetMathLibrary.MakeVector` (`KismetMathLibrary.Conv_IntToDouble` (* (`local.X`) 40)) (`KismetMathLibrary.Conv_IntToDouble` (* (`local.Y`) 40)) (`KismetMathLibrary.Conv_IntToDouble` (* (`local.Z`) 40))) (`self.K2_GetActorLocation`))) "AlwaysSpawn" "MultiplyWithRoot" null null))))))))

(fn `UserConstructionScript`)